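; BP_CharacterBase is a character base Blueprint that drives melee attacks through the Gameplay Ability System.
; It acquires GA_Melee on BeginPlay and activates it by class from the MeleeAttack event.
; When SwordCollider begins overlapping another actor of exactly the BP_Enemy class, it sends itself a Skill.melee.dealDamage gameplay event with that enemy as the payload target.
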(event `self.ReceiveBeginPlay`
  (`self.AquireAbility` "/Game/_DEV/GameplayAbilities/Melee/GA_Melee.GA_Melee_C"))

(event `MeleeAttack`
  (`AbilitySystemComponent.TryActivateAbilityByClass` (`self.AbilitySystemComponent`) "/Game/_DEV/GameplayAbilities/Melee/GA_Melee.GA_Melee_C" true))

(event `self.SwordCollider.OnComponentBeginOverlap`
  (params (OverlappedComponent :type "PrimitiveComponent Object Reference") (OtherActor :type "Actor Object Reference") (OtherComp :type "PrimitiveComponent Object Reference") (OtherBodyIndex :type Integer) (bFromSweep :type Boolean) (SweepResult :type "HitResult Structure (by ref)"))
  ;[1 1 1] Shouldnt reference itself
  (if (!= OtherActor self)
    (if (== (`GameplayStatics.GetObjectClass` OtherActor) "/Game/_DEV/Blueprints/Characters/BP_Enemy.BP_Enemy_C")
      (`AbilitySystemBlueprintLibrary.SendGameplayEventToActor` self (struct :`TagName` "skill.melee.dealDamage") (make `GameplayEventData` (struct) null OtherActor)))))

(fn `UserConstructionScript`)